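; BP_GroundBrake is an overlap-triggered obstacle that checks the player's collection progress when touched by BP_ThirdPersonCharacter.
; If the character's Collected5 flag is set, it zeroes and prints CurrentCollectedAmount, then destroys itself.
; Otherwise it turns on physics simulation for the character's mesh and adds a WBP_Wake widget to the viewport.
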(event Collision|EventActorBeginOverlap
  (params (OtherActor :type Actor%20Object%20Reference))
  (bind _asbp_third_person_character (Utilities|Casting|CastToBP_ThirdPersonCharacter OtherActor))
  (if (Variables|/Game/ThirdPerson/Blueprints/BP_ThirdPersonCharacter.BP_ThirdPersonCharacter_C|GetCollected%205? _asbp_third_person_character)
    (bind _output_get (Variables|/Game/ThirdPerson/Blueprints/BP_ThirdPersonCharacter.BP_ThirdPersonCharacter_C|SetCurrentCollectedAmount _asbp_third_person_character 0))
    (Development|PrintString (Utilities|String|ToString(Integer) _output_get))
    (Actor|DestroyActor)
    (else
      (Physics|SetSimulatePhysics (Variables|/Script/Engine.Character|GetMesh _asbp_third_person_character) true)
      (bind _returnvalue (UserInterface|CreateWidget "/Game/Falling/Widgets/WBP_Wake.WBP_Wake_C"))
      (UserInterface|Viewport|AddtoViewport _returnvalue 0))))

(fn ConstructionScript)